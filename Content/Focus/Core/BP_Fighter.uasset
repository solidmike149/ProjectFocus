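; BP_Fighter is the skeletal-mesh fighter for either the player or enemy side, playing move montages and syncing attribute UI to them.
; On BeginPlay it caches its AnimInstance and builds an AnimationID-to-montage map from its DT_Fighters row's animation table.
; Montage notifies push phase attributes to the game UI: Heat Cost and Focus Recharge update the owner, Damage the opponent.
; Montage completion, or a missing animation, calls CallOnMontageCompleted.
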(event EventBeginPlay
  (bind _asab_mannequin (Utilities|Casting|CastToAB_Mannequin (Components|SkeletalMesh|GetAnimInstance (Variables|Default|GetSkeletalMesh))))
  (Variables|Default|SetAnimInstance _asab_mannequin)
  (CallFunction|SaveAnimations))

(event EventPlayMontage
  (params (MoveCosmetics :type F%20Turn%20Wrapper%20Structure))
  (bind (_animationid _phase) (Utilities|Struct|BreakFTurnWrapper MoveCosmetics))
  (bind (_animationid_2 _phase_2) (Utilities|Struct|BreakFTurnWrapper MoveCosmetics))
  (bind _animations (Variables|Default|GetAnimations))
  (bind _gameuiref (Variables|Default|GetGameUIRef))
  (bind _gameuiref_2 (Variables|Default|GetGameUIRef))
  (bind _gameuiref_3 (Variables|Default|GetGameUIRef))
  (bind _gameuiref_4 (Variables|Default|GetGameUIRef))
  (bind _gameuiref_5 (Variables|Default|GetGameUIRef))
  (bind _gameuiref_6 (Variables|Default|GetGameUIRef))
  (bind _animations_2 (Variables|Default|GetAnimations))
  (bind (_value _returnvalue) (Utilities|Map|Find _animations _animationid_2))
  (bind (_value_2 _returnvalue_2) (Utilities|Map|Find _animations_2 _animationid))
  (switch Utilities|FlowControl|Switch|SwitchonEAttacker (Variables|Default|GetFighterOwner)
    (:NewEnumerator1
      (if _returnvalue
        (bind _notifyname (Animation|Montage|PlayMontage (Variables|Default|GetSkeletalMesh) _value)
          (:OnCompleted
            (Default|CallOnMontageCompleted :!label _label))
          (:OnNotifyBegin
            (switch name _notifyname
              (:HeatCost
                (Utilities|IsValid _gameuiref_4
                  (:Is%20Valid
                    (Default|UpdatePlayerAttributes _gameuiref_4 true (.Value (Utilities|Map|Find _phase_2 "NewEnumerator0"))))))
              (:Damage
                (Utilities|IsValid _gameuiref_5
                  (:Is%20Valid
                    (Default|UpdatePlayerAttributes _gameuiref_5 false (.Value (Utilities|Map|Find _phase_2 "NewEnumerator1"))))))
              (:FocusRecharge
                (Utilities|IsValid _gameuiref_6
                  (:Is%20Valid
                    (Default|UpdatePlayerAttributes _gameuiref_6 true (.Value (Utilities|Map|Find _phase_2 "NewEnumerator2")))))))))
        (else
          (goto _label))))
    (:NewEnumerator2
      (if _returnvalue_2
        (bind _notifyname_2 (Animation|Montage|PlayMontage (Variables|Default|GetSkeletalMesh) _value_2)
          (:OnCompleted
            (Default|CallOnMontageCompleted :!label _label_2))
          (:OnNotifyBegin
            (switch name _notifyname_2
              (:HeatCost
                (Utilities|IsValid _gameuiref
                  (:Is%20Valid
                    (Default|UpdatePlayerAttributes _gameuiref false (.Value (Utilities|Map|Find _phase "NewEnumerator0"))))))
              (:Damage
                (Utilities|IsValid _gameuiref_3
                  (:Is%20Valid
                    (Default|UpdatePlayerAttributes _gameuiref_3 true (.Value (Utilities|Map|Find _phase "NewEnumerator1"))))))
              (:FocusRecharge
                (Utilities|IsValid _gameuiref_2
                  (:Is%20Valid
                    (Default|UpdatePlayerAttributes _gameuiref_2 false (.Value (Utilities|Map|Find _phase "NewEnumerator2")))))))))
        (else
          (goto _label_2))))))

(event EventSetPlayRate
  (params (PlayRate :type Float%20%28single-precision%29))
  (Default|SetPlayRate (Variables|Default|GetAnimInstance) PlayRate))

(fn ConstructionScript)

(fn SaveAnimations
  (bind _returnvalue (Utilities|GetDataTableRow "/Game/Focus/Data/DT_Fighters.DT_Fighters" (Variables|Default|GetFighter%20ID))
    (:then
      (bind _outrownames (DataTable|GetDataTableRowNames (Utilities|Struct|BreakFFighter _returnvalue)))
      (for _array_element _outrownames
        (bind _returnvalue_2 (Utilities|GetDataTableRow (Utilities|Struct|BreakFFighter _returnvalue) _array_element)
          (:then
            (Utilities|Map|Add (Variables|Default|GetAnimations) _array_element (Utilities|Struct|BreakFAnimation _returnvalue_2))))))))