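; Player controller for a networked turn-based fighter, bridging the GameMode, the fight UI and client-side combat playback.
; It sends the fighter ID and three-slot action bar to the server, and sets up UI, animations and characters from DT_Fighters.
; Collected per-segment cosmetics replay as montages in priority order, with notifies driving attribute updates and game over.
; An unfinished BP_Fighter spawn/playback path sits beside the active skeletal-mesh one.
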(event Custom|ClientPostLogin
  ;[1 1 1] Called By GameMode: Initialize UI and Attributes
  (Utilities|FlowControl|Delay 1.0)
  (bind _asbp_game_instance (Utilities|Casting|CastToBP_GameInstance (Game|GetGameInstance)))
  (if (.InState? (Default|GetGameStatus _asbp_game_instance "NewEnumerator3"))
    (GameSetup|SetupGameUI)))

(event Custom|ConfirmActionBar
  (params (Array :type Array%20of%20Names))
  (bind _gamemode_ref (Variables|System|GetGameMode_Ref))
  ;[1 1 1] Send ActionBar To GameMode
  (Networking|SwitchHasAuthority
    (:Authority
      (Utilities|IsValid _gamemode_ref
        (:Is%20Valid
          (Default|ReceiveActionBarIDs _gamemode_ref Array (Variables|/Game/Focus/Core/Net/PS.PS_C|GetPlayerControllerID (Variables|System|GetPlayerState_Ref))))))))

(event Custom|ServerSendIDToGameMode
  (params (FighterID :type Name) (ControllerID :type Integer))
  ;[1 1 1] Sending Fighter Info To GameMode
  (Networking|SwitchHasAuthority
    (:Authority
      (Default|ReceivePlayerFighterID (Variables|System|GetGameMode_Ref) FighterID ControllerID))))

(event Custom|PassSelfToPlayerState
  (params (EnemyStartingFocusMax :type Integer) (EnemyStartingHeatMax :type Integer))
  (Default|InitializeEnemyAttributes (Variables|System|GetPlayerState_Ref) EnemyStartingFocusMax EnemyStartingHeatMax)
  (Variables|/Game/Focus/Core/Net/PS.PS_C|SetOwningPlayerController (Variables|System|GetPlayerState_Ref) self))

(event Custom|SpawnFighters
  (params (FighterID :type Name))
  ;[1 1 1] Spawn Player and Enemy Characters_NEW
  (Utilities|FlowControl|FlipFlop
    (:A
      (bind _returnvalue (Utilities|GetDataTableRow "/Game/Focus/Data/DT_Fighters.DT_Fighters" FighterID)
        (:then
          (bind _returnvalue_2 (Game|SpawnActorfromClass "/Game/Focus/Core/BP_Fighter.BP_Fighter_C" (Math|Transform|MakeTransform "-285.000000,-125.000000, 0" "0, 0, 0" "1,1,1") "Undefined" 0 "NewEnumerator1" 0))
          (Utilities|Array|Add (Variables|Default|GetCharacterObjects) _returnvalue_2))
        (:RowNotFound
          (Development|PrintString "Mesh Not Found"))))
    (:B
      (bind _returnvalue_3 (Utilities|GetDataTableRow "/Game/Focus/Data/DT_Fighters.DT_Fighters" FighterID)
        (:then
          (bind _returnvalue_4 (Game|SpawnActorfromClass "/Game/Focus/Core/BP_Fighter.BP_Fighter_C" (Math|Transform|MakeTransform "-285.000000,125.000000, 0" "0, 0, 0" "1,-1.000000,1") "Undefined" 0 "NewEnumerator2" 0))
          (Utilities|Array|Add (Variables|Default|GetCharacterObjects) _returnvalue_4))
        (:RowNotFound
          (Development|PrintString "Mesh Not Found"))))))

(event Custom|PlayCombatPhase
  (bind _playerstate_ref (Variables|System|GetPlayerState_Ref))
  (bind _playercontrollerid (Variables|/Game/Focus/Core/Net/PS.PS_C|GetPlayerControllerID _playerstate_ref))
  (switch Utilities|FlowControl|Switch|SwitchonEFighter (Utilities|Array|Get(acopy) (Variables|Default|GetPriorities) (Variables|Default|GetLoopIndex))
    (:Fighter0
      (switch int _playercontrollerid
        (:0
          (CallFunction|PlayAnimationsOLD "NewEnumerator1"))
        (:1
          (CallFunction|PlayAnimationsOLD "NewEnumerator2"))))
    (:Fighter1
      (switch int _playercontrollerid
        (:0
          (CallFunction|PlayAnimationsOLD "NewEnumerator2"))
        (:1
          (CallFunction|PlayAnimationsOLD "NewEnumerator1"))))
    (:Both
      (CallFunction|PlayAnimationsOLD "NewEnumerator3"))))

(event Custom|ClientGameOver
  (params (ControllerID :type Integer) (SegmentIndex :type Integer))
  (Variables|Default|SetEndGameSegmentIndex SegmentIndex)
  (Variables|Default|SetDidLost (== ControllerID (Variables|/Game/Focus/Core/Net/PS.PS_C|GetPlayerControllerID (Variables|System|GetPlayerState_Ref)))))

(event Custom|ContinueLoop
  (bind _gameuiref (Variables|Default|GetGameUIRef))
  (Math|Integer|IncrementInt (Variables|Default|GetLoopIndex)
    (:%20%20
      (if (>= (Utilities|Array|LastIndex (Variables|Default|GetPriorities)) (Variables|Default|GetLoopIndex))
        (CallFunction|ContinueCombatPhase)
        (else
          (Variables|Default|SetLoopIndex 0)
          (Utilities|IsValid _gameuiref
            (:Is%20Valid
              (Default|EnterinPlanningMode _gameuiref)
              (Utilities|Array|Clear (Variables|Default|GetTurnCosmeticsPlayer))
              (Utilities|Array|Clear (Variables|Default|GetTurnCosmeticsEnemy))
              (Utilities|Array|Clear (Variables|Default|GetPriorities))
              (Variables|Default|SetCompletedAnimations 0))))))))

(event Custom|WaitForCompletedAnimations
  (switch int (Variables|Default|GetCompletedAnimations)
    (:0
      (Math|Integer|IncrementInt (Variables|Default|GetCompletedAnimations)))
    (:1
      (CallFunction|ContinueLoop)
      (Variables|Default|SetCompletedAnimations 0))))

(event Custom|ContinueCombatPhase
  (bind _gameuiref (Variables|Default|GetGameUIRef))
  (bind _playerstate_ref (Variables|System|GetPlayerState_Ref))
  (bind _playercontrollerid (Variables|/Game/Focus/Core/Net/PS.PS_C|GetPlayerControllerID _playerstate_ref))
  (Utilities|IsValid _gameuiref
    (:Is%20Valid
      (Default|ShowNextSegment _gameuiref (Variables|Default|GetLoopIndex)))
    (:Is%20Not%20Valid
      _))
  (switch Utilities|FlowControl|Switch|SwitchonEFighter (Utilities|Array|Get(acopy) (Variables|Default|GetPriorities) (Variables|Default|GetLoopIndex))
    (:Fighter0
      (switch int _playercontrollerid
        (:0
          (CallFunction|PlayAnimationsOLD "NewEnumerator1"))
        (:1
          (CallFunction|PlayAnimationsOLD "NewEnumerator2"))))
    (:Fighter1
      (switch int _playercontrollerid
        (:0
          (CallFunction|PlayAnimationsOLD "NewEnumerator2"))
        (:1
          (CallFunction|PlayAnimationsOLD "NewEnumerator1"))))
    (:Both
      (CallFunction|PlayAnimationsOLD "NewEnumerator3"))))

(event Custom|CustomEvent
  (params (Attacker :type EAttacker%20Enum :default "NewEnumerator1"))
  (Variables|Default|SetIsEndGame (== (Variables|Default|GetEndGameSegmentIndex) (Variables|Default|GetLoopIndex)))
  (switch Utilities|FlowControl|Switch|SwitchonEAttacker Attacker
    (:NewEnumerator1
      (Class|BPIAnimation|PlayMontage(Message) (Utilities|Array|Get(acopy) (Variables|Default|GetCharacterObjects)) (Utilities|Array|Get(acopy) (Variables|Default|GetTurnCosmeticsPlayer) (Variables|Default|GetLoopIndex))))
    (:NewEnumerator2
      (Class|BPIAnimation|PlayMontage(Message) (Utilities|Array|Get(acopy) (Variables|Default|GetCharacterObjects) 1) (Utilities|Array|Get(acopy) (Variables|Default|GetTurnCosmeticsEnemy) (Variables|Default|GetLoopIndex))))))

(event Custom|CollectCombatCosmetics
  (params (Attacker :type EAttacker%20Enum :default "NewEnumerator0") (Segment%20Phase :type ESegmentPhase%20Enum :default "NewEnumerator0") (Attributes :type Array%20of%20F%20Attribute%20Structures) (Name :type Name) (SegmentIndex :type Integer))
  (switch Utilities|FlowControl|Switch|SwitchonEAttacker Attacker
    (:NewEnumerator1
      (if (Utilities|Enum|Equal(Enum) "NewEnumerator1" Segment%20Phase)
        (if (Utilities|Array|IsValidIndex (Variables|Default|GetTurnCosmeticsEnemy) SegmentIndex) :!label _label
          (Utilities|Map|Add (Utilities|Struct|BreakFTurnWrapper (Utilities|Array|Get(acopy) (Variables|Default|GetTurnCosmeticsEnemy) SegmentIndex)) Segment%20Phase (Utilities|Struct|MakeFPhaseWrapper Attributes))
          (else
            (Utilities|Array|Add (Variables|Default|GetTurnCosmeticsEnemy) (Utilities|Struct|MakeFTurnWrapper Name (Utilities|Map|MakeMap Segment%20Phase (Utilities|Struct|MakeFPhaseWrapper Attributes))))))
        (else
          (if (Utilities|Array|IsValidIndex (Variables|Default|GetTurnCosmeticsPlayer) SegmentIndex) :!label _label_2
            (Utilities|Map|Add (Utilities|Struct|BreakFTurnWrapper (Utilities|Array|Get(acopy) (Variables|Default|GetTurnCosmeticsPlayer) SegmentIndex)) Segment%20Phase (Utilities|Struct|MakeFPhaseWrapper Attributes))
            (else
              (Utilities|Array|Add (Variables|Default|GetTurnCosmeticsPlayer) (Utilities|Struct|MakeFTurnWrapper Name (Utilities|Map|MakeMap Segment%20Phase (Utilities|Struct|MakeFPhaseWrapper Attributes)))))))))
    (:NewEnumerator2
      (if (Utilities|Enum|Equal(Enum) Segment%20Phase "NewEnumerator1")
        (goto _label_2)
        (else
          (goto _label))))))

(event Custom|GameOver
  (params (ControllerID :type Integer) (SegmentIndex :type Integer))
  (CallFunction|ClientGameOver ControllerID SegmentIndex))

(event Custom|SpawnCharacters_OLD
  (params (FighterID :type Name))
  ;[1 1 1] Spawn Player and Enemy Characters_OLD
  (Utilities|FlowControl|FlipFlop
    (:A
      (bind _returnvalue (Utilities|GetDataTableRow "/Game/Focus/Data/DT_Fighters.DT_Fighters" FighterID)
        (:then
          (bind _returnvalue_2 (Game|SpawnActorfromClass "/Script/Engine.SkeletalMeshActor" (Math|Transform|MakeTransform "-140.000000,910.000000,-70.000000" "0,-90.000000, 0" "1,1,1") "Undefined" 0 0))
          (Utilities|Array|Add (Variables|Default|GetCharacters) _returnvalue_2)
          (Class|SkinnedMeshComponent|SetSkeletalMesh (Variables|/Script/Engine.SkeletalMeshActor|GetSkeletalMeshComponent _returnvalue_2) (Utilities|Struct|BreakFFighter _returnvalue) true)
          (Class|SkeletalMeshComponent|SetAnimClass (Variables|/Script/Engine.SkeletalMeshActor|GetSkeletalMeshComponent _returnvalue_2) "/Game/Focus/Art/Characters/Mannequin/Animations/AB_Mannequin.AB_Mannequin_C"))
        (:RowNotFound
          (Development|PrintString "Mesh Not Found"))))
    (:B
      (bind _returnvalue_3 (Utilities|GetDataTableRow "/Game/Focus/Data/DT_Fighters.DT_Fighters" FighterID)
        (:then
          (bind _returnvalue_4 (Game|SpawnActorfromClass "/Script/Engine.SkeletalMeshActor" (Math|Transform|MakeTransform "140.000000,910.000000,-70.000000" "0,-90.000000, 0" "1,-1.000000,1") "Undefined" 0 0))
          (Utilities|Array|Add (Variables|Default|GetCharacters) _returnvalue_4)
          (Class|SkinnedMeshComponent|SetSkeletalMesh (Variables|/Script/Engine.SkeletalMeshActor|GetSkeletalMeshComponent _returnvalue_4) (Utilities|Struct|BreakFFighter _returnvalue_3) true)
          (Class|SkeletalMeshComponent|SetAnimClass (Variables|/Script/Engine.SkeletalMeshActor|GetSkeletalMeshComponent _returnvalue_4) "/Game/Focus/Art/Characters/Mannequin/Animations/AB_Mannequin.AB_Mannequin_C"))
        (:RowNotFound
          (Development|PrintString "Mesh Not Found"))))))

(event Custom|PlayAnimation)

(event Custom|PlayAnimations_OLD
  (params (Attacker :type EAttacker%20Enum :default "NewEnumerator1"))
  (bind _turncosmeticsplayer (Variables|Default|GetTurnCosmeticsPlayer))
  (bind _animationmap (Variables|Default|GetAnimationMap))
  (bind _loopindex (Variables|Default|GetLoopIndex))
  (bind _animationmap_2 (Variables|Default|GetAnimationMap))
  (bind _animationmap_3 (Variables|Default|GetAnimationMap))
  (bind _gameuiref (Variables|Default|GetGameUIRef))
  (bind _loopindex_2 (Variables|Default|GetLoopIndex))
  (bind _gameuiref_2 (Variables|Default|GetGameUIRef))
  (bind _gameuiref_3 (Variables|Default|GetGameUIRef))
  (bind _loopindex_3 (Variables|Default|GetLoopIndex))
  (bind _turncosmeticsenemy (Variables|Default|GetTurnCosmeticsEnemy))
  (bind _gameuiref_4 (Variables|Default|GetGameUIRef))
  (bind _gameuiref_5 (Variables|Default|GetGameUIRef))
  (bind _gameuiref_6 (Variables|Default|GetGameUIRef))
  (bind _gameuiref_7 (Variables|Default|GetGameUIRef))
  (bind _animationmap_4 (Variables|Default|GetAnimationMap))
  (bind _gameuiref_8 (Variables|Default|GetGameUIRef))
  (bind _gameuiref_9 (Variables|Default|GetGameUIRef))
  (bind _loopindex_4 (Variables|Default|GetLoopIndex))
  (bind _turncosmeticsenemy_2 (Variables|Default|GetTurnCosmeticsEnemy))
  (bind _gameuiref_10 (Variables|Default|GetGameUIRef))
  (bind _gameuiref_11 (Variables|Default|GetGameUIRef))
  (bind _gameuiref_12 (Variables|Default|GetGameUIRef))
  (bind _turncosmeticsplayer_2 (Variables|Default|GetTurnCosmeticsPlayer))
  (bind _loopindex_5 (Variables|Default|GetLoopIndex))
  (bind _animationmap_5 (Variables|Default|GetAnimationMap))
  (bind _gameuiref_13 (Variables|Default|GetGameUIRef))
  (bind _turncosmeticsplayer_3 (Variables|Default|GetTurnCosmeticsPlayer))
  (bind _gameuiref_14 (Variables|Default|GetGameUIRef))
  (bind _gameuiref_15 (Variables|Default|GetGameUIRef))
  (bind _animationmap_6 (Variables|Default|GetAnimationMap))
  (bind _loopindex_6 (Variables|Default|GetLoopIndex))
  (bind _turncosmeticsenemy_3 (Variables|Default|GetTurnCosmeticsEnemy))
  (bind _gameuiref_16 (Variables|Default|GetGameUIRef))
  (bind _gameuiref_17 (Variables|Default|GetGameUIRef))
  (bind _gameuiref_18 (Variables|Default|GetGameUIRef))
  (bind _output (Utilities|Array|Get(acopy) _turncosmeticsenemy_2 _loopindex_4))
  (bind _output_2 (Utilities|Array|Get(acopy) _turncosmeticsplayer_2 _loopindex_5))
  (bind _output_3 (Utilities|Array|Get(acopy) _turncosmeticsenemy_3 _loopindex_6))
  (bind _output_4 (Utilities|Array|Get(acopy) _turncosmeticsplayer_3 _loopindex_2))
  (bind _output_5 (Utilities|Array|Get(acopy) _turncosmeticsplayer _loopindex))
  (bind _output_6 (Utilities|Array|Get(acopy) _turncosmeticsenemy _loopindex_3))
  (bind (_animationid _phase) (Utilities|Struct|BreakFTurnWrapper _output_3))
  (bind (_animationid_2 _phase_2) (Utilities|Struct|BreakFTurnWrapper _output_5))
  (bind (_animationid_3 _phase_3) (Utilities|Struct|BreakFTurnWrapper _output_6))
  (bind (_animationid_4 _phase_4) (Utilities|Struct|BreakFTurnWrapper _output))
  (bind (_animationid_5 _phase_5) (Utilities|Struct|BreakFTurnWrapper _output_4))
  (bind (_animationid_6 _phase_6) (Utilities|Struct|BreakFTurnWrapper _output_2))
  (bind (_value _returnvalue) (Utilities|Map|Find _animationmap _animationid_2))
  (bind (_value_2 _returnvalue_2) (Utilities|Map|Find _animationmap_2 _animationid_3))
  (bind (_value_3 _returnvalue_3) (Utilities|Map|Find _animationmap_3 _animationid_5))
  (bind (_value_4 _returnvalue_4) (Utilities|Map|Find _animationmap_5 _animationid_6))
  (bind (_value_5 _returnvalue_5) (Utilities|Map|Find _animationmap_6 _animationid))
  (bind (_value_6 _returnvalue_6) (Utilities|Map|Find _animationmap_4 _animationid_4))
  (Variables|Default|SetIsEndGame (== (Variables|Default|GetEndGameSegmentIndex) (Variables|Default|GetLoopIndex)))
  (switch Utilities|FlowControl|Switch|SwitchonEAttacker Attacker
    (:NewEnumerator1
      (if _returnvalue
        (bind _notifyname (Animation|Montage|PlayMontage (Variables|/Script/Engine.SkeletalMeshActor|GetSkeletalMeshComponent (Utilities|Array|Get(acopy) (Variables|Default|GetCharacters))) _value)
          (:OnCompleted
            (if _returnvalue_5 :!label _label
              (bind _notifyname_2 (Animation|Montage|PlayMontage (Variables|/Script/Engine.SkeletalMeshActor|GetSkeletalMeshComponent (Utilities|Array|Get(acopy) (Variables|Default|GetCharacters) 1)) _value_5)
                (:OnCompleted
                  (CallFunction|ContinueLoop :!label _label_2))
                (:OnNotifyBegin
                  (switch name _notifyname_2
                    (:HeatCost
                      (Utilities|IsValid _gameuiref_16
                        (:Is%20Valid
                          (Default|UpdatePlayerAttributes _gameuiref_16 false (.Value (Utilities|Map|Find _phase "NewEnumerator0"))))))
                    (:Damage
                      (Utilities|IsValid _gameuiref_17
                        (:Is%20Valid
                          (Default|UpdatePlayerAttributes _gameuiref_17 true (.Value (Utilities|Map|Find _phase "NewEnumerator1")))
                          (if (Variables|Default|GetIsEndGame)
                            (Default|GameOver _gameuiref_17 (Variables|Default|GetDidLost))))))
                    (:FocusRecharge
                      (Utilities|IsValid _gameuiref_18
                        (:Is%20Valid
                          (Default|UpdatePlayerAttributes _gameuiref_18 false (.Value (Utilities|Map|Find _phase "NewEnumerator2")))))))))
              (else
                (goto _label_2))))
          (:OnNotifyBegin
            (switch name _notifyname
              (:HeatCost
                (Utilities|IsValid _gameuiref_13
                  (:Is%20Valid
                    (Default|UpdatePlayerAttributes _gameuiref_13 true (.Value (Utilities|Map|Find _phase_2 "NewEnumerator0"))))))
              (:Damage
                (Utilities|IsValid _gameuiref_14
                  (:Is%20Valid
                    (Default|UpdatePlayerAttributes _gameuiref_14 false (.Value (Utilities|Map|Find _phase_2 "NewEnumerator1")))
                    (if (Variables|Default|GetIsEndGame)
                      (Default|GameOver _gameuiref_14 (Variables|Default|GetDidLost))))))
              (:FocusRecharge
                (Utilities|IsValid _gameuiref_15
                  (:Is%20Valid
                    (Default|UpdatePlayerAttributes _gameuiref_15 true (.Value (Utilities|Map|Find _phase_2 "NewEnumerator2")))))))))
        (else
          (goto _label))))
    (:NewEnumerator2
      (if _returnvalue_2
        (bind _notifyname_3 (Animation|Montage|PlayMontage (Variables|/Script/Engine.SkeletalMeshActor|GetSkeletalMeshComponent (Utilities|Array|Get(acopy) (Variables|Default|GetCharacters) 1)) _value_2)
          (:OnCompleted
            (if _returnvalue_3 :!label _label_3
              (bind _notifyname_4 (Animation|Montage|PlayMontage (Variables|/Script/Engine.SkeletalMeshActor|GetSkeletalMeshComponent (Utilities|Array|Get(acopy) (Variables|Default|GetCharacters))) _value_3)
                (:OnCompleted
                  (CallFunction|ContinueLoop :!label _label_4))
                (:OnNotifyBegin
                  (switch name _notifyname_4
                    (:HeatCost
                      (Utilities|IsValid _gameuiref_2
                        (:Is%20Valid
                          (Default|UpdatePlayerAttributes _gameuiref_2 true (.Value (Utilities|Map|Find _phase_5 "NewEnumerator0"))))))
                    (:Damage
                      (Utilities|IsValid _gameuiref_6
                        (:Is%20Valid
                          (Default|UpdatePlayerAttributes _gameuiref_6 false (.Value (Utilities|Map|Find _phase_5 "NewEnumerator1")))
                          (if (Variables|Default|GetIsEndGame)
                            (Default|GameOver _gameuiref_6 (Variables|Default|GetDidLost))))))
                    (:FocusRecharge
                      (Utilities|IsValid _gameuiref_3
                        (:Is%20Valid
                          (Default|UpdatePlayerAttributes _gameuiref_3 true (.Value (Utilities|Map|Find _phase_5 "NewEnumerator2")))))))))
              (else
                (goto _label_4))))
          (:OnNotifyBegin
            (switch name _notifyname_3
              (:HeatCost
                (Utilities|IsValid _gameuiref_4
                  (:Is%20Valid
                    (Default|UpdatePlayerAttributes _gameuiref_4 false (.Value (Utilities|Map|Find _phase_3 "NewEnumerator0"))))))
              (:Damage
                (Utilities|IsValid _gameuiref_5
                  (:Is%20Valid
                    (Default|UpdatePlayerAttributes _gameuiref_5 true (.Value (Utilities|Map|Find _phase_3 "NewEnumerator1")))
                    (if (Variables|Default|GetIsEndGame)
                      (Default|GameOver _gameuiref_5 (Variables|Default|GetDidLost))))))
              (:FocusRecharge
                (Utilities|IsValid _gameuiref
                  (:Is%20Valid
                    (Default|UpdatePlayerAttributes _gameuiref false (.Value (Utilities|Map|Find _phase_3 "NewEnumerator2")))))))))
        (else
          (goto _label_3))))
    (:NewEnumerator3
      (for _array_element (Variables|Default|GetCharacters)
        (Utilities|FlowControl|MultiGate false true -1
          (:Out%200
            (if _returnvalue_4
              (bind _notifyname_5 (Animation|Montage|PlayMontage (Variables|/Script/Engine.SkeletalMeshActor|GetSkeletalMeshComponent _array_element) _value_4)
                (:OnCompleted
                  (CallFunction|WaitforCompletedAnimations :!label _label_5))
                (:OnNotifyBegin
                  (switch name _notifyname_5
                    (:HeatCost
                      (Utilities|IsValid _gameuiref_7
                        (:Is%20Valid
                          (Default|UpdatePlayerAttributes _gameuiref_7 true (.Value (Utilities|Map|Find _phase_6 "NewEnumerator0"))))))
                    (:Damage
                      (Utilities|IsValid _gameuiref_8
                        (:Is%20Valid
                          (Default|UpdatePlayerAttributes _gameuiref_8 false (.Value (Utilities|Map|Find _phase_6 "NewEnumerator1"))))))
                    (:FocusRecharge
                      (Utilities|IsValid _gameuiref_9
                        (:Is%20Valid
                          (Default|UpdatePlayerAttributes _gameuiref_9 true (.Value (Utilities|Map|Find _phase_6 "NewEnumerator2")))))))))
              (else
                (goto _label_5))))
          (:Out%201
            (if _returnvalue_6
              (bind _notifyname_6 (Animation|Montage|PlayMontage (Variables|/Script/Engine.SkeletalMeshActor|GetSkeletalMeshComponent _array_element) _value_6)
                (:OnCompleted
                  (CallFunction|WaitforCompletedAnimations :!label _label_6))
                (:OnNotifyBegin
                  (switch name _notifyname_6
                    (:HeatCost
                      (Utilities|IsValid _gameuiref_10
                        (:Is%20Valid
                          (Default|UpdatePlayerAttributes _gameuiref_10 false (.Value (Utilities|Map|Find _phase_4 "NewEnumerator0"))))))
                    (:Damage
                      (Utilities|IsValid _gameuiref_11
                        (:Is%20Valid
                          (Default|UpdatePlayerAttributes _gameuiref_11 true (.Value (Utilities|Map|Find _phase_4 "NewEnumerator1"))))))
                    (:FocusRecharge
                      (Utilities|IsValid _gameuiref_12
                        (:Is%20Valid
                          (Default|UpdatePlayerAttributes _gameuiref_12 false (.Value (Utilities|Map|Find _phase_4 "NewEnumerator2")))))))))
              (else
                (goto _label_6)))))))))

(event Custom|Server_ConfirmActionBar
  (params (Array :type Array%20of%20Names))
  ;[1 1 1] Send ActionBar To GameMode
  (CallFunction|ConfirmActionBar Array))

(event Custom|SetCombatMode
  ;[1 1 1] Changing Match Phase on UI
  (Default|EnterinCombatMode (Variables|Default|GetGameUIRef)))

(event Custom|SetCountdownTimer
  (params (Time :type Integer))
  ;[1 1 1] Decrementing Countdown Time
  (GameSetup|SetTimer Time))

(event Custom|ReceivePriority
  (params (Priorities :type Array%20of%20EFighter%20Enums :default "NoFighter"))
  (Variables|Default|SetPriorities Priorities))

(event Custom|FillActionBarEnemy
  (params (Moves :type Array%20of%20F%20Move%20Structures))
  (Default|PassMovestoActionBar (Variables|Default|GetGameUIRef) Moves))

(event Custom|TurnReady
  ;[1 1 1] Send ActionBar To GameMode
  (CallFunction|ServerConfirmActionBar (Variables|Default|GetActionBarIDs))
  (Variables|Default|SetActionBarIDs (Utilities|Array|MakeArray "None" "None" "None")))

(event Custom|InitializeEnemy
  (params (EnemyFighterID :type Name))
  (bind _gameuiref (Variables|Default|GetGameUIRef))
  (bind _playerstate_ref (Variables|System|GetPlayerState_Ref))
  (bind (_startingfocus_max _startingheat_max) (Default|GetStartingAttributes _playerstate_ref))
  (if (Pawn|IsLocalPlayerController)
    (Utilities|IsValid _gameuiref
      (:Is%20Valid
        (bind _returnvalue (Utilities|GetDataTableRow "/Game/Focus/Data/DT_Fighters.DT_Fighters" EnemyFighterID)
          (:then
            (Default|InitializeMovesPanel _gameuiref false (.Moveset (Utilities|Struct|BreakFFighter _returnvalue)))
            (Default|InitializeAttributes _gameuiref _startingfocus_max _startingheat_max (.StartingFocus (Utilities|Struct|BreakFFighter _returnvalue)) (.StartingHeat (Utilities|Struct|BreakFFighter _returnvalue)))
            (CallFunction|SaveAnimations false EnemyFighterID)
            (CallFunction|SpawnCharactersOLD EnemyFighterID)
            (CallFunction|PassSelftoPlayerState (.StartingFocus (Utilities|Struct|BreakFFighter _returnvalue)) (.StartingHeat (Utilities|Struct|BreakFFighter _returnvalue)))))))))

(event EventBeginPlay
  (bind _asbp_game_instance (Utilities|Casting|CastToBP_GameInstance (Game|GetGameInstance)))
  (Variables|Default|SetFighter%20ID (Variables|/Game/Focus/Core/BP_GameInstance.BP_GameInstance_C|GetFighterID _asbp_game_instance))
  (Input|DisableInput self)
  (bind _returnvalue (Actor|GetActorOfClass "/Script/CinematicCamera.CineCameraActor"))
  (Game|Player|SetViewTargetwithBlend self _returnvalue 0.0 "VTBlend_Linear" 0.0 false)
  (Utilities|FlowControl|Delay 0.8)
  (bind _asgs (Utilities|Casting|CastToGS (Game|GetGameState)))
  (Variables|System|SetGameState_Ref _asgs)
  (bind _asps (Utilities|Casting|CastToPS (Variables|GetPlayerState self)))
  (Variables|System|SetPlayerState_Ref _asps)
  ;[1 1 1] Saving Server References
  (Networking|SwitchHasAuthority
    (:Authority
      (bind _asgm (Utilities|Casting|CastToGM (Game|GetGameMode)))
      (bind _output_get (Variables|System|SetGameMode_Ref _asgm))
      (EventDispatchers|BindEventtoOnPlayerDefeat _output_get (delegate Custom|GameOver)))
    (:Remote
      (CallFunction|SaveAnimations true (Variables|Default|GetFighter%20ID))
      (Utilities|IsValid (Variables|System|GetPlayerState_Ref)
        (:Is%20Valid
          (CallFunction|ServerSendIDtoGameMode (Variables|Default|GetFighter%20ID) (Variables|/Game/Focus/Core/Net/PS.PS_C|GetPlayerControllerID (Variables|System|GetPlayerState_Ref)))
          (CallFunction|SpawnCharactersOLD (Variables|Default|GetFighter%20ID)))))))

(fn ConstructionScript)

(fn UpdateActionBar
  (params (Adding :type Boolean) (Segment :type Integer) (MoveID :type Name))
  (if Adding
    (Utilities|Array|SetArrayElem (Variables|Default|GetActionBarIDs) Segment MoveID)
    (else
      (Utilities|Array|SetArrayElem (Variables|Default|GetActionBarIDs) Segment "")))
  (return))

(fn SetupGameUI
  (if (Pawn|IsLocalPlayerController)
    (bind _returnvalue (UserInterface|CreateWidget "/Game/Focus/Core/UI/WBP_FightWidget.WBP_FightWidget_C"))
    (bind _output_get (Variables|Default|SetGameUIRef _returnvalue))
    (UserInterface|Viewport|AddtoViewport _output_get 0)
    (Variables|/Game/Focus/Core/UI/WBP_FightWidget.WBP_FightWidget_C|SetPlayerController_Ref _output_get self)
    (EventDispatchers|BindEventtoReadytoPlayCombat _output_get (EventDispatchers|CreateEvent :!event Custom|PlayCombatPhase))
    (bind _returnvalue_2 (Utilities|GetDataTableRow "/Game/Focus/Data/DT_Fighters.DT_Fighters" (Variables|Default|GetFighter%20ID))
      (:then
        (Default|InitializeMovesPanel _output_get true (Utilities|Struct|BreakFFighter _returnvalue_2))
        (return)))))

(fn SetTimer
  (params (Time :type Integer))
  (Utilities|IsValid (Variables|Game|GetCountdownTimerWidget)
    (:Is%20Valid
      _)
    (:Is%20Not%20Valid
      (bind _returnvalue (UserInterface|CreateWidget "/Game/Focus/Core/UI/WBP_Countdown.WBP_Countdown_C"))
      (bind _output_get (Variables|Game|SetCountdownTimerWidget _returnvalue))
      (UserInterface|Viewport|AddtoViewport _output_get 0)))
  (bind _output_get_2 (Variables|/Game/Focus/Core/UI/WBP_Countdown.WBP_Countdown_C|SetTimer _output_get Time))
  (if (< _output_get_2 1)
    (Widget|RemovefromParent (Variables|Game|GetCountdownTimerWidget))
    (return)
    (else
      (return))))

(fn IsinOverheat
  (return (Default|IsinOverheat (Variables|System|GetPlayerState_Ref))))

(fn SaveAnimations
  (params (IsPlayer :type Boolean) (InFighterID :type Name))
  (if IsPlayer
    (bind _returnvalue (Utilities|GetDataTableRow "/Game/Focus/Data/DT_Fighters.DT_Fighters" InFighterID :!label _label)
      (:then
        (bind _outrownames (DataTable|GetDataTableRowNames (Utilities|Struct|BreakFFighter _returnvalue)))
        (for _array_element _outrownames
          (bind _returnvalue_2 (Utilities|GetDataTableRow (Utilities|Struct|BreakFFighter _returnvalue) _array_element)
            (:then
              (Utilities|Map|Add (Variables|Default|GetAnimationMap) _array_element (Utilities|Struct|BreakFAnimation _returnvalue_2)))))
        (return)))
    (elif (Utilities|Name|NotEqual(Name) InFighterID (Variables|Default|GetFighter%20ID))
      (goto _label))))

(fn DebugCosmetics
  (params (Array :type Array%20of%20F%20Turn%20Wrapper%20Structures))
  (for _array_element Array
    (Development|PrintString (Utilities|String|ToString(Name) (.AnimationID (Utilities|Struct|BreakFTurnWrapper _array_element))))
    (bind _keys (Utilities|Map|Keys (.Phase (Utilities|Struct|BreakFTurnWrapper _array_element))))
    (LocalVariables|SetKeys _keys)
    (bind _values (Utilities|Map|Values (.Phase (Utilities|Struct|BreakFTurnWrapper _array_element))))
    (LocalVariables|SetValues _values)
    (for _index (range 0 (Utilities|Map|Length (.Phase (Utilities|Struct|BreakFTurnWrapper _array_element))))
      (Development|PrintString (Utilities|String|Append "Phase " (Utilities|String|EnumtoString (Utilities|Array|Get(acopy) (LocalVariables|GetKeys)))))
      (for _array_element_2 (.attributes (Utilities|Array|Get(acopy) (LocalVariables|GetValues)))
        (Development|PrintString (Utilities|String|Append "Value " (Utilities|String|ToString(Integer) (.value _array_element_2)) (Utilities|String|EnumtoString (.type _array_element_2)))))))
  (return))