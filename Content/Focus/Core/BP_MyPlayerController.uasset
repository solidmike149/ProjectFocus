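; Player controller for a turn-based networked fight, linking the local UI to the GameMode and GameState.
; It switches to a cine camera, builds the fight and countdown widgets, and forwards phase, attribute and game-over updates to them.
; Planned moves fill an action bar array, sent through a server event to the GameMode when the turn is ready.
; Fighter identity and move tables are hardcoded to Kusha for the player and Levine for the enemy.
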(event Custom|ClientPostLogin
  ;[1 1 1] Called By GameMode: Initialize UI and Attributes
  (Utilities|FlowControl|Delay 1.0)
  (bind _asbp_game_instance (Utilities|Casting|CastToBP_GameInstance (Game|GetGameInstance)))
  (if (.InState? (Default|GetGameStatus _asbp_game_instance "NewEnumerator3"))
    (GameSetup|SetupGameUI)))

(event Custom|ConfirmActionBar
  (params (Array :type Array%20of%20Names))
  (bind _gamemode_ref (Variables|System|GetGameMode_Ref))
  ;[1 1 1] Send ActionBar To GameMode
  (Networking|SwitchHasAuthority
    (:Authority
      (Utilities|IsValid _gamemode_ref
        (:Is%20Valid
          (Default|ReceiveActionBarIDs _gamemode_ref Array (Variables|/Game/Focus/Core/Net/PS.PS_C|GetPlayerControllerID (Variables|System|GetPlayerState_Ref))))))))

(event Custom|UpdateGameUI
  (params (UIToModify :type UIToModify%20Enum :default "NewEnumerator0") (AttributeToChange :type EAttribute%20Enum :default "NewEnumerator0") (Combo :type ECombo%20Enum :default "NewEnumerator6") (NewValue :type Integer) (IsDamage :type Boolean))
  (bind _gameui_ref (Variables|Default|GetGameUI_Ref))
  (Utilities|IsValid _gameui_ref
    (:Is%20Valid
      (Default|UpdateAttributes _gameui_ref UIToModify AttributeToChange Combo NewValue IsDamage))))

(event Custom|Server_ConfirmActionBar
  (params (Array :type Array%20of%20Names))
  ;[1 1 1] Send ActionBar To GameMode
  (CallFunction|ConfirmActionBar Array))

(event Custom|SetCombatMode
  ;[1 1 1] Changing Match Phase on UI
  (Default|EnterinCombatMode (Variables|Default|GetGameUI_Ref)))

(event Custom|SetCountdownTimer
  (params (Time :type Integer))
  ;[1 1 1] Decrementing Countdown Time
  (GameSetup|SetTimer Time))

(event Custom|SetPlanningMode
  (Default|EnterinPlanningMode (Variables|Default|GetGameUI_Ref)))

(event Custom|GameOver
  (Default|GameOver (Variables|Default|GetGameUI_Ref)))

(event Custom|TurnReady
  ;[1 1 1] Send ActionBar To GameMode
  (CallFunction|ServerConfirmActionBar (Variables|Default|GetActionBarIDs))
  (for _array_element (Variables|Default|GetActionBarIDs)
    (Development|PrintString (Utilities|String|ToString(Name) _array_element)))
  (Variables|Default|SetActionBarIDs (Utilities|Array|MakeArray "None" "None" "None")))

(event Custom|InitializeUIValuesEvent
  (params (EnemyStartingHeat :type Integer) (EnemyStartingFocus :type Integer) (EnemyFighterID :type Name))
  (bind _gameui_ref (Variables|Default|GetGameUI_Ref))
  (bind _playerstate_ref (Variables|System|GetPlayerState_Ref))
  (bind (_startingheat_max _startingfocus_max) (Default|GetStartingAttributes _playerstate_ref))
  (if (Pawn|IsLocalPlayerController)
    (Utilities|IsValid _gameui_ref
      (:Is%20Valid
        (bind (_starting_focus _starting_heat) (CallFunction|FindFighterInfobyName EnemyFighterID))
        (Default|InitializeValues _gameui_ref _startingheat_max _startingfocus_max _starting_focus _starting_heat)))))

(event EventBeginPlay
  (bind _asbp_game_instance (Utilities|Casting|CastToBP_GameInstance (Game|GetGameInstance)))
  (Variables|Default|SetFighter%20ID (Variables|/Game/Focus/Core/BP_GameInstance.BP_GameInstance_C|GetFighterID _asbp_game_instance))
  (Input|DisableInput self)
  (bind _returnvalue (Actor|GetActorOfClass "/Script/CinematicCamera.CineCameraActor"))
  (Game|Player|SetViewTargetwithBlend self _returnvalue 0.0 "VTBlend_Linear" 0.0 false)
  (Utilities|FlowControl|Delay 0.8)
  (bind _asgs (Utilities|Casting|CastToGS (Game|GetGameState)))
  (bind _output_get (Variables|System|SetGameState_Ref _asgs))
  (EventDispatchers|BindEventtoOnNotifyPlanningMode _output_get (delegate Custom|SetPlanningMode))
  (bind _asps (Utilities|Casting|CastToPS (Variables|GetPlayerState self)))
  (Variables|System|SetPlayerState_Ref _asps)
  ;[1 1 1] Saving Server References
  (Networking|SwitchHasAuthority
    (:Authority
      (bind _asgm (Utilities|Casting|CastToGM (Game|GetGameMode)))
      (bind _output_get_2 (Variables|System|SetGameMode_Ref _asgm))
      (EventDispatchers|BindEventtoOnPlayerDefeat _output_get_2 (delegate Custom|GameOver))
      ;[1 1 1] Sending Fighter Info To GameMode
      (Default|ReceivePlayerFighterID (Variables|System|GetGameMode_Ref) "Kusha" (Variables|/Game/Focus/Core/Net/PS.PS_C|GetPlayerControllerID (Variables|System|GetPlayerState_Ref))))))

(fn ConstructionScript)

(fn AddtoActionBarArray
  (params (Segment :type Integer) (MoveID :type Name))
  (Utilities|Array|SetArrayElem (Variables|Default|GetActionBarIDs) Segment MoveID))

(fn SetupGameUI
  (if (Pawn|IsLocalPlayerController)
    (bind _returnvalue (UserInterface|CreateWidget "/Game/Focus/Core/UI/WBP_FightWidget.WBP_FightWidget_C"))
    (bind _output_get (Variables|Default|SetGameUI_Ref _returnvalue))
    (UserInterface|Viewport|AddtoViewport _output_get 0)
    (Variables|/Game/Focus/Core/UI/WBP_FightWidget.WBP_FightWidget_C|SetPlayerController_Ref _output_get self)
    (Default|InitializeMovesPanel _output_get true "/Game/Focus/Data/DT_Kusha.DT_Kusha")
    (return)))

(fn SetTimer
  (params (Time :type Integer))
  (Utilities|IsValid (Variables|Game|GetCountdownTimerWidget)
    (:Is%20Valid
      _)
    (:Is%20Not%20Valid
      (bind _returnvalue (UserInterface|CreateWidget "/Game/Focus/Core/UI/WBP_Countdown.WBP_Countdown_C"))
      (bind _output_get (Variables|Game|SetCountdownTimerWidget _returnvalue))
      (UserInterface|Viewport|AddtoViewport _output_get 0)))
  (bind _output_get_2 (Variables|/Game/Focus/Core/UI/WBP_Countdown.WBP_Countdown_C|SetTimer _output_get Time))
  (if (< _output_get_2 1)
    (Widget|RemovefromParent (Variables|Game|GetCountdownTimerWidget))
    (return)
    (else
      (return))))

(fn IsinOverheat
  (return (Default|IsinOverheat (Variables|System|GetPlayerState_Ref))))

(fn FindFighterInfobyName
  (params (FighterID :type Name))
  (bind _array_element (Utilities|Array|ForEachLoopwithBreak (Variables|/Script/ProjectFocus.FighterInfoDataAsset|GetFighters (Variables|Default|GetDataAsset)) :!label _label)
    (:LoopBody
      (if (Utilities|Name|Equal(Name) (.FighterID (Utilities|Struct|BreakFighter _array_element)) FighterID)
        (goto _label Break)))
    (:Completed
      (Default|InitializeMovesPanel (Variables|Default|GetGameUI_Ref) false "/Game/Focus/Data/DT_Levine.DT_Levine")
      (return (.StartingFocus (Utilities|Struct|BreakFighter _array_element)) (.StartingHeat (Utilities|Struct|BreakFighter _array_element))))))